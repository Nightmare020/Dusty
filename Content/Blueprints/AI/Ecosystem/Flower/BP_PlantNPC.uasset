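; BP_PlantNPC is a plant NPC for the AI ecosystem with configurable size and color.
; The Construction Script maps the Size option to a uniform relative scale on MSkeletalMesh, ranging from slightly smaller to slightly larger than default.
; It then maps the Color option to a pink, green, purple or blue material instance on that mesh.
; The Event Graph holds only disabled placeholder events, so this Blueprint's graphs add no runtime behavior.
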(event EventBeginPlay)

(event Collision|EventActorBeginOverlap
  (params (OtherActor :type Actor%20Object%20Reference)))

(event EventTick
  (params (DeltaSeconds :type Float%20%28single-precision%29)))

(fn ConstructionScript
  (switch Utilities|FlowControl|Switch|SwitchonEM_FlowerSizes (Variables|Default|GetSize)
    (:NewEnumerator0
      (Transformation|SetRelativeScale3D (Variables|Default|Getm_SkeletalMesh) "0.800000,0.800000,0.800000"))
    (:NewEnumerator1
      (Transformation|SetRelativeScale3D (Variables|Default|Getm_SkeletalMesh) "0.900000,0.900000,0.900000"))
    (:NewEnumerator2
      (Transformation|SetRelativeScale3D (Variables|Default|Getm_SkeletalMesh) "1.000000,1.000000,1.000000"))
    (:NewEnumerator3
      (Transformation|SetRelativeScale3D (Variables|Default|Getm_SkeletalMesh) "1.100000,1.100000,1.100000"))
    (:NewEnumerator4
      (Transformation|SetRelativeScale3D (Variables|Default|Getm_SkeletalMesh) "1.200000,1.200000,1.200000")))
  (switch Utilities|FlowControl|Switch|SwitchonEM_PlantColors (Variables|Default|GetColor)
    (:NewEnumerator0
      (Rendering|Material|SetMaterial (Variables|Default|Getm_SkeletalMesh) 0 "/Game/MATERIALS/MI/CustomNPC/MI_PlantNpcPink.MI_PlantNpcPink"))
    (:NewEnumerator1
      (Rendering|Material|SetMaterial (Variables|Default|Getm_SkeletalMesh) 0 "/Game/MATERIALS/MI/CustomNPC/MI_PlantNPCGreen.MI_PlantNPCGreen"))
    (:NewEnumerator2
      (Rendering|Material|SetMaterial (Variables|Default|Getm_SkeletalMesh) 0 "/Game/MATERIALS/MI/CustomNPC/MI_PlantNPCPurple.MI_PlantNPCPurple"))
    (:NewEnumerator3
      (Rendering|Material|SetMaterial (Variables|Default|Getm_SkeletalMesh) 0 "/Game/MATERIALS/MI/CustomNPC/MI_PlantNPCBlue.MI_PlantNPCBlue"))))