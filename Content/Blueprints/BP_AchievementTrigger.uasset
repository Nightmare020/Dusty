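; Trigger actor that writes an online achievement when an actor of a configured class overlaps it.
; On overlap it caches the first player controller's achievements, then looks up the configured AchievementID in that cache.
; It writes progress only if the ID is found with no progress above zero.
; Wrong actor class, cache failure, missing ID and already-earned cases just print debug strings.
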(event `self.ReceiveActorBeginOverlap`
  (params (OtherActor :type "Actor Object Reference"))
  (bind _returnvalue (`GameplayStatics.GetPlayerController` 0))
  (if (`GameplayStatics.ObjectIsA` OtherActor (`self.ActorToEnter`))
    (`AchievementQueryCallbackProxy.CacheAchievements` _returnvalue
      (:`OnSuccess`
        (bind (_bfoundid _progress) (`AchievementBlueprintLibrary.GetCachedAchievementProgress` _returnvalue (`self.Achievement ID`)))
        (if _bfoundid
          (if (> _progress 0.0)
            (`KismetSystemLibrary.PrintString` "already gotten")
            (else
              (`AchievementWriteCallbackProxy.WriteAchievementProgress` (`GameplayStatics.GetPlayerController` 0) (`self.Achievement ID`))))
          (else
            (`KismetSystemLibrary.PrintString` "Achievement not found"))))
      (:`OnFailure`
        (`KismetSystemLibrary.PrintString` "FailCache")))
    (else
      (`KismetSystemLibrary.PrintString` "Not Actor"))))

(fn `UserConstructionScript`)