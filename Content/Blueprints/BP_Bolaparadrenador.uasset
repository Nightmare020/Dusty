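; BP_Bolaparadrenador is a sphere actor that drives position and radius material parameters, likely for a spherical masking effect.
; Every Tick, it writes the Sphere component's world location to the "Position" vector parameter and its Radius variable to the "Radius" scalar parameter.
; The Construction Script makes the same writes, so the values also update when the actor is constructed or edited.
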(event `self.ReceiveActorBeginOverlap`
  (params (OtherActor :type "Actor Object Reference")))

(event `self.ReceiveTick`
  (params (DeltaSeconds :type "Float (single-precision)"))
  (`KismetMaterialLibrary.SetVectorParameterValue` null "Position" (`KismetMathLibrary.Conv_VectorToLinearColor` (`SceneComponent.K2_GetComponentLocation` (`self.Sphere`))))
  (`KismetMaterialLibrary.SetScalarParameterValue` null "Radius" (`self.Radius`)))

(fn `UserConstructionScript`
  (`KismetMaterialLibrary.SetVectorParameterValue` null "Position" (`KismetMathLibrary.Conv_VectorToLinearColor` (`SceneComponent.K2_GetComponentLocation` (`self.Sphere`))))
  (`KismetMaterialLibrary.SetScalarParameterValue` null "Radius" (`self.Radius`)))