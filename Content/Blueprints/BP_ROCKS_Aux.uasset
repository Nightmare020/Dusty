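; BP_ROCKS_Aux is a rock prop that tumbles continuously with a randomized look and spin.
; On BeginPlay it picks one of two low mid-rock meshes at random and rolls a per-axis rotation rate between Min and Max.
; Tick adds that rate, scaled by DeltaSeconds, to the mesh's world roll, pitch and yaw for frame-rate-independent spinning.
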(event `self.ReceiveBeginPlay`
  (bind _staticmesh (`self.StaticMesh`))
  (bind _min (`self.Min`))
  (bind _max (`self.Max`))
  (set `self.RandomRotation` (`KismetMathLibrary.MakeRotator` (`KismetMathLibrary.RandomFloatInRange` _min _max) (`KismetMathLibrary.RandomFloatInRange` _min _max) (`KismetMathLibrary.RandomFloatInRange` _min _max)))
  (if (`KismetMathLibrary.RandomBool`)
    (`StaticMeshComponent.SetStaticMesh` _staticmesh "/Game/MESHES/ROCKS/SM_MidRock_low_01.SM_MidRock_low_01")
    (else
      (`StaticMeshComponent.SetStaticMesh` _staticmesh "/Game/MESHES/ROCKS/SM_MidRock_low_05.SM_MidRock_low_05"))))

(event `self.ReceiveTick`
  (params (DeltaSeconds :type "Float (single-precision)"))
  (bind _staticmesh (`self.StaticMesh`))
  (bind (_returnvalue_roll _returnvalue_pitch _returnvalue_yaw) (`KismetMathLibrary.BreakRotator` (`SceneComponent.K2_GetComponentRotation` _staticmesh)))
  (`SceneComponent.K2_SetWorldRotation` _staticmesh (`KismetMathLibrary.MakeRotator` (+ _returnvalue_roll (* (.roll (`self.RandomRotation`)) DeltaSeconds)) (+ _returnvalue_pitch (* (.pitch (`self.RandomRotation`)) DeltaSeconds)) (+ _returnvalue_yaw (* (.yaw (`self.RandomRotation`)) DeltaSeconds))) false false))

(fn `UserConstructionScript`)