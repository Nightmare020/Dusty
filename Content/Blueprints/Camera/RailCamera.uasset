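; A trigger-volume Blueprint that switches the player's view to a separate camera while BP_DustyCharacter is inside its Box.
; On begin overlap it blends to the ViewTarget camera and enables look-at tracking on the player pawn.
; On end overlap it blends back to the pawn and turns tracking off.
; Despite the RailCamera name, the Blueprint contains no rail movement logic.
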(event `self.Box.OnComponentBeginOverlap`
  (params (OverlappedComponent :type "PrimitiveComponent Object Reference") (OtherActor :type "Actor Object Reference") (OtherComp :type "PrimitiveComponent Object Reference") (OtherBodyIndex :type Integer) (bFromSweep :type Boolean) (SweepResult :type "HitResult Structure (by ref)"))
  (cast `/Game/Blueprints/Characters/BP_DustyCharacter` OtherActor)
  (`PlayerController.SetViewTargetWithBlend` (`GameplayStatics.GetPlayerController` 0) (`self.ViewTarget`) 1.0 "VTBlend_Linear" 0.0 false)
  (set `CineCameraActor.LookatTrackingSettings` (make `CameraLookatTrackingSettings` true false 0.0 (`|ConvertAsset` (`GameplayStatics.GetPlayerPawn` 0))) (`self.ViewTarget`)))

(event `self.Box.OnComponentEndOverlap`
  (params (OverlappedComponent :type "PrimitiveComponent Object Reference") (OtherActor :type "Actor Object Reference") (OtherComp :type "PrimitiveComponent Object Reference") (OtherBodyIndex :type Integer))
  (cast `/Game/Blueprints/Characters/BP_DustyCharacter` OtherActor)
  (`PlayerController.SetViewTargetWithBlend` (`GameplayStatics.GetPlayerController` 0) (`GameplayStatics.GetPlayerPawn` 0) 1.0 "VTBlend_Linear" 0.0 false)
  (set `CineCameraActor.LookatTrackingSettings` (make `CameraLookatTrackingSettings` false) (`self.ViewTarget`)))

(fn `UserConstructionScript`)