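; Character Blueprint for Dusty, providing material setup plus grass, audio and achievement hooks.
; BeginPlay disables capsule physics and puts a dynamic material on mesh slot 1.
; Callable events publish the capsule position to the MPC_WIND parameter collection for grass, move the audio listener onto Dusty, and write achievement progress after caching, printing on failure.
; Tick is empty, and pole-bone debug drawing is disconnected.
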(event `self.ReceiveTick`
  (params (DeltaSeconds :type "Float (single-precision)")))

(event `self.UpdateGrassEffect`
  (params (_color :type "LinearColor Structure (by ref)"))
  (`KismetMaterialLibrary.SetVectorParameterValue` "/Game/MATERIALS/MPC_CURVES/MPC_WIND.MPC_WIND" "PlayerPos" (`KismetMathLibrary.Conv_VectorToLinearColor` (`SceneComponent.K2_GetComponentLocation` (`self.CapsuleComponent`)))))

(event `self.ReceiveBeginPlay`
  (`PrimitiveComponent.SetSimulatePhysics` (`self.CapsuleComponent`) false)
  (bind _returnvalue (`self.SetDustyDynamicMaterial` (`PrimitiveComponent.GetMaterial` (`self.Mesh`) 1)))
  (`PrimitiveComponent.SetMaterial` (`self.Mesh`) 1 _returnvalue))

(event `self.ChangeAudioListener`
  ;[1 1 1] Change Audio listener to Dusty
  (`PlayerController.SetAudioListenerOverride` :`self` (`GameplayStatics.GetPlayerController` 0) :`AttachToComponent` (`self.AudioListener`)))

(event `self.UnlockAchievement`
  (params (AchievementId :type Name) (Progress :type "Float (single-precision)"))
  (bind _returnvalue (`GameplayStatics.GetPlayerController` 0))
  (`AchievementQueryCallbackProxy.CacheAchievements` _returnvalue
    (:`OnSuccess`
      (bind _bfoundid (`AchievementBlueprintLibrary.GetCachedAchievementProgress` _returnvalue AchievementId))
      (if _bfoundid
        (`AchievementWriteCallbackProxy.WriteAchievementProgress` (`GameplayStatics.GetPlayerController` 0) AchievementId Progress)
        (else
          (`KismetSystemLibrary.PrintString` (`KismetStringLibrary.Conv_NameToString` AchievementId)))))
    (:`OnFailure`
      (`KismetSystemLibrary.PrintString` "FailCache"))))

(fn `UserConstructionScript`)