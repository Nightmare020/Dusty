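; Physics-driven plant actor that pulls itself back toward its starting position when displaced.
; BeginPlay records the world location of Cube as the rest point.
; Each Tick applies a spring-like force to MMesh, proportional to Cube's offset from that point.
; Within a small radius of rest, it zeroes the mesh's linear velocity every frame in place of damping.
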(event `self.ReceiveBeginPlay`
  (set `self.InitialPlanPos` (`SceneComponent.K2_GetComponentLocation` (`self.Cube`))))

(event `self.ReceiveTick`
  (params (DeltaSeconds :type "Float (single-precision)"))
  (bind _returnvalue (- (`self.InitialPlanPos`) (`SceneComponent.K2_GetComponentLocation` (`self.Cube`))))
  (`PrimitiveComponent.AddForce` (`self.m_mesh`) (* _returnvalue 6000.0) "None" false)
  (if (<= (`KismetMathLibrary.VSize` _returnvalue) 10.0)
    (`PrimitiveComponent.SetAllPhysicsLinearVelocity` (`self.m_mesh`) (0.0 0.0 0.0) false)))

(fn `UserConstructionScript`)