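; Test double-door Blueprint for the hieroglyphics puzzle that slides two door panels apart when activated.
; Activate runs a fast looping timer on OpenDoors, then clears it after a short delay.
; Each tick nudges DoorLeft and DoorRight in opposite directions along local Y without sweeping.
; An older approach that hid the doors and disabled their collision remains disconnected and never runs.
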(event `self.BP_Activate`
  (`KismetSystemLibrary.K2_SetTimer` null "OpenDoors" 0.025 true)
  (`KismetSystemLibrary.Delay` 1.2)
  (`KismetSystemLibrary.K2_ClearTimer` null "OpenDoors"))

(event `OpenDoors`
  (`SceneComponent.K2_AddLocalOffset` (`self.DoorLeft`) (0.0 5.0 0.0) false false)
  (`SceneComponent.K2_AddLocalOffset` (`self.DoorRight`) (0.0 -5.0 0.0) false false))

(fn `UserConstructionScript`)