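; BP_FloorTool is a construction-script tool that builds floors from spline mesh components laid along an editable spline, optionally closed as a loop.
; Each segment gets MeshesPerPoint components, each with a random mesh from the SplineMesh array, two shared materials and query-and-physics collision.
; Copies shift sideways by a Y-only iteration offset scaled by the tangent's rotated normal, with positions and tangents divided by InitialScale to compensate for component scale.
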(fn `AddFloorMeshComponent`
  (params (`Spline Index` :type Integer))
  (bind (_returnvalue_x _returnvalue_y) (`KismetMathLibrary.BreakVector` (`self.Get Current Mesh Offset` 1)))
  (bind (_returnvalue_x_2 _returnvalue_y_2) (`KismetMathLibrary.BreakVector` (`self.Get Current Mesh Offset` 1)))
  (bind _initialscale (`self.InitialScale`))
  (bind _spline (`self.Spline`))
  (bind _next_spline_point (`self.Next Spline Point`))
  (bind _returnvalue (`SplineComponent.GetTangentAtSplinePoint` _spline `Spline Index` "World"))
  (bind _returnvalue_2 (`SplineComponent.GetTangentAtSplinePoint` _spline _next_spline_point "World"))
  (bind (_returnvalue_x_3 _returnvalue_y_3) (`KismetMathLibrary.BreakVector` (* _returnvalue_y (`KismetMathLibrary.Normal` (`KismetMathLibrary.RotateAngleAxis` _returnvalue 90.0 (`self.Axis`))))))
  (bind (_returnvalue_x_4 _returnvalue_y_4) (`KismetMathLibrary.BreakVector` (* _returnvalue_y_2 (`KismetMathLibrary.Normal` (`KismetMathLibrary.RotateAngleAxis` _returnvalue_2 90.0 (`self.Axis`))))))
  (bind _returnvalue_3 (`AddComponent|NODE_AddSplineMeshComponent-0` :`RelativeTransform` (`KismetMathLibrary.MakeTransform` (0.0 0.0 0.0) (struct) (`self.InitialScale`))))
  (`KismetArrayLibrary.Array_Add` (`self.RootsMesh`) _returnvalue_3)
  (`StaticMeshComponent.SetStaticMesh` _returnvalue_3 (`self.GetSplinePointMesh` `Spline Index`))
  (`PrimitiveComponent.SetMaterial` _returnvalue_3 0 (`self.SplineMaterial_1`))
  (`PrimitiveComponent.SetMaterial` _returnvalue_3 1 (`self.SplineMaterial_2`))
  (`SplineMeshComponent.SetForwardAxis` _returnvalue_3 (`self.Spline Axis`) true)
  (`SceneComponent.K2_SetRelativeRotation` _returnvalue_3 (`self.World Rotation`) false false)
  (`SplineMeshComponent.SetStartAndEnd` _returnvalue_3 (/ (+ (`KismetMathLibrary.MakeVector` 0.0 _returnvalue_y_3) (`SplineComponent.GetLocationAtSplinePoint` _spline `Spline Index` "Local")) _initialscale) (/ _returnvalue _initialscale) (/ (+ (`KismetMathLibrary.MakeVector` 0.0 _returnvalue_y_4) (`SplineComponent.GetLocationAtSplinePoint` _spline _next_spline_point "Local")) _initialscale) (/ _returnvalue_2 _initialscale) true)
  (`PrimitiveComponent.SetCollisionEnabled` _returnvalue_3 "QueryAndPhysics"))

(fn `Get Current Mesh Offset`
  (params (Point :type Integer :default 1))
  (returns (ReturnValue :type "Vector Structure"))
  (bind _returnvalue (- (`self.Current Mesh Per Point`) Point))
  (if (> _returnvalue 0)
    (return (* (`self.Mesh Iteration Offset`) _returnvalue))
    (else
      (return (0.0 0.0 0.0)))))

(fn `GetSplinePointMesh`
  (params (`Spline Point` :type Integer))
  (returns (Mesh :type "StaticMesh Object Reference"))
  (return (`KismetArrayLibrary.Array_Random` (`self.Spline Mesh`))))

(fn `UserConstructionScript`
  (locals (`Spline Points` :type Integer))
  (bind _spline (`self.Spline`))
  (bind _returnvalue (`SplineComponent.GetNumberOfSplinePoints` _spline))
  (bind _returnvalue_2 (- _returnvalue 1))
  (if (`self.Loop`)
    (`SplineComponent.SetClosedLoop` _spline true true)
    (set `local.Spline Points` _returnvalue_2)
    (else
      (`SplineComponent.SetClosedLoop` _spline false true)
      (set `local.Spline Points` (- _returnvalue 2))))
  (for _index (range (+ (`local.Spline Points`) 1))
    (if (and (== _index _returnvalue_2) (`self.Loop`))
      (set `self.Next Spline Point` 0)
      (else
        (set `self.Next Spline Point` (+ _index 1))))
    (set `self.Current Mesh Per Point` (`self.Meshes Per Point`))
    (while (> (`self.Current Mesh Per Point`) 0)
      (`self.AddFloorMeshComponent` _index)
      (`/Engine/EditorBlueprintResources/StandardMacros.DecrementInt` (`self.Current Mesh Per Point`)))))