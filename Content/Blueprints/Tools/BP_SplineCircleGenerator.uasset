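; Editor tool actor that builds a circular or helical spline from radius, point count and per-point height.
; The construction script adds spline points, then cycles them through four quadrant positions, raising each by Height times its index.
; Each point gets a perpendicular tangent scaled by Radius × 1.656854, approximating a true circle with four points per turn, with Height as the tangent's Z.
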(fn `SetTangent`
  (params (X :type "Float (double-precision)") (Y :type "Float (double-precision)"))
  (bind _returnvalue (* (`self.Radius`) 1.656854))
  (set `self.Tangent` (`KismetMathLibrary.MakeVector` (* X _returnvalue) (* Y _returnvalue) (`self.Height`))))

(fn `SetVector`
  (params (X :type "Float (double-precision)") (Y :type "Float (double-precision)"))
  (set `self.Location` (`KismetMathLibrary.MakeVector` X Y (* (`self.Height_Index`) (`self.Height`))))
  (return))

(fn `UserConstructionScript`
  (for _ (range (+ (- (`self.Points`) 3) 1))
    (`SplineComponent.AddSplinePoint` (`self.Spline`) (`KismetMathLibrary.Vector_Zero`) "Local" true))
  (for _index (range (+ (`SplineComponent.GetNumberOfSplinePoints` (`self.Spline`)) 1))
    (set `self.Height_Index` _index)
    (switch `int` (`self.Rotation_Index`)
      (:`0`
        (`self.SetVector` (* (`self.Radius`) 1.0))
        (`self.SetTangent` 0.0 1.0))
      (:`1`
        (`self.SetVector` 0.0 (* (`self.Radius`) 1.0))
        (`self.SetTangent` -1.0))
      (:`2`
        (`self.SetVector` (* (`self.Radius`) -1.0))
        (`self.SetTangent` 0.0 -1.0))
      (:`3`
        (`self.SetVector` 0.0 (* (`self.Radius`) -1.0))
        (`self.SetTangent` 1.0)))
    (`SplineComponent.SetLocationAtSplinePoint` (`self.Spline`) (`self.Height_Index`) (`self.Location`) "Local" true)
    (`SplineComponent.SetTangentAtSplinePoint` (`self.Spline`) (`self.Height_Index`) (`self.Tangent`) "Local" true)
    (bind _result (`/Engine/EditorBlueprintResources/StandardMacros.IncrementInt` (`self.Rotation_Index`))
      (:`  `
        (if (> _result 3)
          (set `self.Rotation_Index` 0))))))