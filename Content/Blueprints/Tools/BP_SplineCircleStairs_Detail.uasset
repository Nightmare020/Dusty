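; Construction-script tool that builds circular or spiral stairs from spline meshes along a spline.
; When the CreateCIrcle flag is set, CreateSpline clears it and rebuilds the spline from eight repeating positions around Radius, rising by Height per point, with scaled tangents.
; Each segment becomes a flat, collidable spline mesh stepped up by Height, its cross-section scaled from the mesh bounds so each step is Height thick.
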(fn `SetTangent`
  (params (X :type "Float (double-precision)") (Y :type "Float (double-precision)"))
  (bind _returnvalue (* (`self.Radius`) 1.656854))
  (set `self.Tangent` (`KismetMathLibrary.MakeVector` (* X _returnvalue) (* Y _returnvalue) (`self.Height`))))

(fn `SetVector`
  (params (X :type "Float (double-precision)") (Y :type "Float (double-precision)"))
  (set `self.Location` (`KismetMathLibrary.MakeVector` X Y (* (`self.Height_Index`) (`self.Height`))))
  (return))

(fn `UserConstructionScript`
  (locals (CurrentHeight :type "Float (double-precision)"))
  (bind _radius (`self.Radius`))
  (bind _radius_2 (`self.Radius`))
  (bind _radius_3 (`self.Radius`))
  (bind _radius_4 (`self.Radius`))
  (bind _spline (`self.Spline`))
  (bind _initialscale (`self.InitialScale`))
  (bind _returnvalue (`SplineComponent.GetNumberOfSplinePoints` (`self.Spline`)))
  (bind _returnvalue_2 (/ (/ (`self.Height`) 2.0) (.z (`.BoxExtent` (`KismetMathLibrary.BreakBoxSphereBounds` (`StaticMesh.GetBounds` (`self.Static Mesh`)))))))
  (if (`self.CreateCIrcle`)
    (set `self.CreateCIrcle` false)
    (`SplineComponent.ClearSplinePoints` (`self.Spline`) true)
    (for _ (range (+ (`self.Points`) 1))
      (`SplineComponent.AddSplinePoint` (`self.Spline`) (`KismetMathLibrary.Vector_Zero`) "Local" true))
    (for _index (range (+ (`SplineComponent.GetNumberOfSplinePoints` (`self.Spline`)) 1))
      (set `self.Height_Index` _index)
      (switch `int` (`self.Rotation_Index`)
        (:`0`
          (`self.SetVector` (* (`self.Radius`) 1.0))
          (`self.SetTangent` 0.0 1.0))
        (:`1`
          (`self.SetVector` (* _radius_3 0.7) (* _radius_3 0.7))
          (`self.SetTangent` 0.0 1.0))
        (:`2`
          (`self.SetVector` 0.0 (* (`self.Radius`) 1.0))
          (`self.SetTangent` -1.0))
        (:`3`
          (`self.SetVector` (* _radius_4 -0.7) (* _radius_4 0.7))
          (`self.SetTangent` -1.0))
        (:`4`
          (`self.SetVector` (* (`self.Radius`) -1.0))
          (`self.SetTangent` 0.0 -1.0))
        (:`5`
          (`self.SetVector` (* _radius_2 -0.7) (* _radius_2 -0.7))
          (`self.SetTangent` 0.0 -1.0))
        (:`6`
          (`self.SetVector` 0.0 (* (`self.Radius`) -1.0))
          (`self.SetTangent` 1.0))
        (:`7`
          (`self.SetVector` (* _radius 0.7) (* _radius -0.7))
          (`self.SetTangent` 0.0 1.0)))
      (`SplineComponent.SetLocationAtSplinePoint` (`self.Spline`) (`self.Height_Index`) (`self.Location`) "Local" true)
      (`SplineComponent.SetTangentAtSplinePoint` (`self.Spline`) (`self.Height_Index`) (`self.Tangent`) "Local" true)
      (bind _result (`/Engine/EditorBlueprintResources/StandardMacros.IncrementInt` (`self.Rotation_Index`))
        (:`  `
          (if (> _result 7)
            (set `self.Rotation_Index` 0))))))
  (if (>= _returnvalue 2)
    (for _index_2 (range (+ (- _returnvalue 2) 1))
      (bind _output_get (set `local.CurrentHeight` (* (`KismetMathLibrary.Conv_IntToDouble` _index_2) (`self.Height`))))
      (bind _returnvalue_3 (`AddComponent|NODE_AddSplineMeshComponent-0` :`RelativeTransform` (`KismetMathLibrary.MakeTransform` (`KismetMathLibrary.MakeVector` 0.0 0.0 _output_get) (struct) (`self.InitialScale`))))
      (`StaticMeshComponent.SetStaticMesh` _returnvalue_3 (`self.Static Mesh`))
      (`PrimitiveComponent.SetMaterial` _returnvalue_3 0 (`self.Mesh Material`))
      (`SplineMeshComponent.SetForwardAxis` _returnvalue_3 (`self.Spline Axis`) true)
      (`SplineMeshComponent.SetEndScale` _returnvalue_3 (`KismetMathLibrary.MakeVector2D` 1.0 _returnvalue_2) true)
      (`SplineMeshComponent.SetStartScale` _returnvalue_3 (`KismetMathLibrary.MakeVector2D` 1.0 _returnvalue_2) true)
      (bind _returnvalue_4 (+ _index_2 1))
      (`SplineMeshComponent.SetStartAndEnd` _returnvalue_3 (`KismetMathLibrary.MakeVector` (.x (/ (`SplineComponent.GetLocationAtSplinePoint` _spline _index_2 "Local") _initialscale)) (.y (/ (`SplineComponent.GetLocationAtSplinePoint` _spline _index_2 "Local") _initialscale))) (`KismetMathLibrary.MakeVector` (.x (/ (`SplineComponent.GetTangentAtSplinePoint` _spline _index_2 "Local") _initialscale)) (.y (/ (`SplineComponent.GetTangentAtSplinePoint` _spline _index_2 "Local") _initialscale))) (`KismetMathLibrary.MakeVector` (.x (/ (`SplineComponent.GetLocationAtSplinePoint` _spline _returnvalue_4 "Local") _initialscale)) (.y (/ (`SplineComponent.GetLocationAtSplinePoint` _spline _returnvalue_4 "Local") _initialscale))) (`KismetMathLibrary.MakeVector` (.x (/ (`SplineComponent.GetTangentAtSplinePoint` _spline _returnvalue_4 "Local") _initialscale)) (.y (/ (`SplineComponent.GetTangentAtSplinePoint` _spline _returnvalue_4 "Local") _initialscale))) true)
      (`PrimitiveComponent.SetCollisionEnabled` _returnvalue_3 "QueryAndPhysics"))))