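; Spline mesh tool that builds a chain of mesh segments along an editable spline in the Construction Script, optionally as a closed loop.
; Each segment not listed in PointsToDissapear gets a collidable SplineMeshComponent with two materials, configurable axis, rotation and scale-compensated tangents.
; Segments step up in Z by Height unless Roots is set.
; GetSplinePointMesh and the empty AddExtraMeshes act as hooks for per-segment variation.
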(fn `AddExtraMeshes`
  (params (`Spline Mesh component` :type "SplineMeshComponent Object Reference")))

(fn `GetSplinePointMesh`
  (params (`Spline Point` :type Integer))
  (returns (Mesh :type "StaticMesh Object Reference"))
  (return (`self.Spline Mesh`)))

(fn `UserConstructionScript`
  (locals (`Spline Points` :type Integer) (CanLoop :type Boolean))
  (bind _current_spline_point (`self.Current Spline Point`))
  (bind _spline (`self.Spline`))
  (bind _current_spline_point_2 (`self.Current Spline Point`))
  (bind _next_spline_point (`self.Next Spline Point`))
  (bind _initialscale (`self.InitialScale`))
  (bind _spline_2 (`self.Spline`))
  (bind _returnvalue (`SplineComponent.GetNumberOfSplinePoints` _spline_2))
  (bind _returnvalue_2 (- _returnvalue 1))
  (if (`self.Loop`)
    (`SplineComponent.SetClosedLoop` _spline_2 true true)
    (set `local.Spline Points` _returnvalue_2)
    (else
      (`SplineComponent.SetClosedLoop` _spline_2 false true)
      (set `local.Spline Points` (- _returnvalue 2))))
  (for _index (range (+ (`local.Spline Points`) 1))
    (set `self.Current Spline Point` _index)
    (set `local.CanLoop` true)
    (for _array_element (`self.PointsToDissapear`)
      (if (== _array_element (`self.Current Spline Point`))
        (set `local.CanLoop` false)
        (break)))
    (if (`local.CanLoop`)
      (if (and (== (`self.Current Spline Point`) _returnvalue_2) (`self.Loop`))
        (set `self.Next Spline Point` 0)
        (else
          (set `self.Next Spline Point` (+ _current_spline_point 1))))
      (bind _returnvalue_3 (`AddComponent|NODE_AddSplineMeshComponent-0` :`RelativeTransform` (`KismetMathLibrary.MakeTransform` (`KismetMathLibrary.MakeVector` 0.0 0.0 (`KismetMathLibrary.Conv_IntToDouble` (* (* _current_spline_point (`self.Height`)) (not (`self.Roots`))))) (struct) (`self.InitialScale`))))
      (`KismetArrayLibrary.Array_Add` (`self.RootsMesh`) _returnvalue_3)
      (`StaticMeshComponent.SetStaticMesh` _returnvalue_3 (`self.GetSplinePointMesh` (`self.Current Spline Point`)))
      (`PrimitiveComponent.SetMaterial` _returnvalue_3 0 (`self.SplineMaterial_1`))
      (`PrimitiveComponent.SetMaterial` _returnvalue_3 1 (`self.SplineMaterial_2`))
      (`SplineMeshComponent.SetForwardAxis` _returnvalue_3 (`self.Spline Axis`) true)
      (`SceneComponent.K2_SetRelativeRotation` _returnvalue_3 (`self.World Rotation`) false false)
      (`SplineMeshComponent.SetStartAndEnd` _returnvalue_3 (/ (`SplineComponent.GetLocationAtSplinePoint` _spline _current_spline_point_2 "Local") _initialscale) (/ (`SplineComponent.GetTangentAtSplinePoint` _spline _current_spline_point_2 "Local") _initialscale) (/ (`SplineComponent.GetLocationAtSplinePoint` _spline _next_spline_point "Local") _initialscale) (/ (`SplineComponent.GetTangentAtSplinePoint` _spline _next_spline_point "Local") _initialscale) true)
      (`PrimitiveComponent.SetCollisionEnabled` _returnvalue_3 "QueryAndPhysics")
      (`self.AddExtraMeshes` _returnvalue_3))))