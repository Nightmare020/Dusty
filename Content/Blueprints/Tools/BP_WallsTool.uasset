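; Spline-based wall building tool that extends a parent spline tool with mesh variants and scattered wall decorations.
; The construction script keeps the weight array sized to the variants; each point uses its mapped mesh (parent fallback) or the highest weighted random roll.
; AddExtraMeshes walks an X/Y grid on each segment, randomly spawning either broken shiny rock meshes with rotation jitter or shelf child actors, gated by an appearance chance.
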(fn `AddExtraMeshes`
  (params (`Spline Mesh component` :type "SplineMeshComponent Object Reference"))
  (locals (Index :type Integer))
  (bind (_min _max) (`StaticMeshComponent.GetLocalBounds` `Spline Mesh component`))
  (bind (_returnvalue_location _returnvalue_rotation _returnvalue_scale) (`KismetMathLibrary.BreakTransform` (`SceneComponent.GetRelativeTransform` `Spline Mesh component`)))
  (bind _spline (`self.Spline`))
  (bind _spline_2 (`self.Spline`))
  (bind _returnvalue (`SplineComponent.GetDistanceAlongSplineAtSplinePoint` _spline_2 (`self.Current Spline Point`)))
  (bind _returnvalue_2 (`KismetMathLibrary.MakeVector` 0.0 0.0 (.z _min)))
  (bind _returnvalue_3 (+ _returnvalue (* (- (`SplineComponent.GetDistanceAlongSplineAtSplinePoint` _spline_2 (`self.Next Spline Point`)) _returnvalue) 0.5)))
  (bind _returnvalue_4 (`KismetMathLibrary.MakeTransform` (+ (`SplineComponent.GetLocationAtDistanceAlongSpline` _spline _returnvalue_3 "Local") (+ (* (/ (- (`KismetMathLibrary.MakeVector` 0.0 0.0 (.z _max)) _returnvalue_2) (+ (`self.Replications on Y`) 1)) (+ (`local.Index`) 1)) _returnvalue_2)) (`SplineComponent.GetRotationAtDistanceAlongSpline` _spline _returnvalue_3 "Local") _returnvalue_scale))
  (set `local.Index` (- (* (`self.Replications on X`) (`self.Replications on Y`)) 1))
  (while (>= (`local.Index`) 0)
    (if (<= (`KismetMathLibrary.RandomFloatInRange` 0.0 1.0) (`self.PercentageToAppear`))
      (if (`KismetMathLibrary.RandomBool`)
        (bind _returnvalue_5 (`AddComponent|NODE_AddStaticMeshComponent-1` :`RelativeTransform` _returnvalue_4))
        (`SceneComponent.K2_SetRelativeRotation` _returnvalue_5 (`KismetMathLibrary.MakeRotator` (+ (.roll (`SceneComponent.RelativeRotation` _returnvalue_5)) (`KismetMathLibrary.RandomFloatInRange` -15.0 15.0)) (+ (.pitch (`SceneComponent.RelativeRotation` _returnvalue_5)) (`KismetMathLibrary.RandomFloatInRange` -15.0 15.0)) (+ (.yaw (`SceneComponent.RelativeRotation` _returnvalue_5)) (`KismetMathLibrary.RandomFloatInRange` 0.0 15.0))) false false)
        (`StaticMeshComponent.SetStaticMesh` _returnvalue_5 (`KismetArrayLibrary.Array_Random` (`self.ShinyRockBrokenMesh`)))
        (`/Engine/EditorBlueprintResources/StandardMacros.DecrementInt` (`local.Index`))
        (else
          (bind _returnvalue_6 (`AddComponent|NODE_AddChildActorComponent-0` :`RelativeTransform` _returnvalue_4))
          (`ChildActorComponent.SetChildActorClass` _returnvalue_6 (`KismetArrayLibrary.Array_Random` (`self.ShelfClasses`)))
          (`/Engine/EditorBlueprintResources/StandardMacros.DecrementInt` (`local.Index`))))
      (else
        (`/Engine/EditorBlueprintResources/StandardMacros.DecrementInt` (`local.Index`))))))

(fn `GetSplinePointMesh`
  (params (`Spline Point` :type Integer))
  (returns (Mesh :type "StaticMesh Object Reference"))
  (locals (MapPoint :type Integer) (BiggestRandom :type Integer) (BiggestRandom_keys :type "Float (double-precision)"))
  (bind (_value _returnvalue) (`BlueprintMapLibrary.Map_Find` (`self.MeshVariantsPoints`) (+ `Spline Point` 1)))
  (bind _output (`|GetArrayItem` (`self.MeshVariants`) (`local.MapPoint`)))
  (if (not (`self.RandomVarianPoints`))
    (if _returnvalue
      (set `local.MapPoint` _value)
      (`/Engine/EditorBlueprintResources/StandardMacros.IsValid` _output
        (:`Is Valid`
          (return _output))
        (:`Is Not Valid`
          _)))
    (return (`parent.GetSplinePointMesh` 0))
    (else
      (`BlueprintMapLibrary.Map_Clear` (`self.MeshVariantsPercentageAux`))
      (for (_array_element _array_index) (`self.MeshVariantsPercentage`)
        (`BlueprintMapLibrary.Map_Add` (`self.MeshVariantsPercentageAux`) (`KismetMathLibrary.RandomFloatInRange` 0.0 (+ _array_element (* 0.5 (== _array_element 0.0)))) _array_index))
      (bind _keys (`BlueprintMapLibrary.Map_Keys` (`self.MeshVariantsPercentageAux`)))
      (for (_array_element_2 _array_index_2) _keys
        (if (> _array_element_2 (`local.BiggestRandom_keys`))
          (set `local.BiggestRandom_keys` _array_element_2)
          (set `local.BiggestRandom` _array_index_2)))
      (return (`|GetArrayItem` (`self.MeshVariants`) (`local.BiggestRandom`))))))

(fn `UserConstructionScript`
  (`parent.UserConstructionScript`)
  (`KismetArrayLibrary.Array_Resize` (`self.MeshVariantsPercentage`) (`KismetArrayLibrary.Array_Length` (`self.MeshVariants`))))