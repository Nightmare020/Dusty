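; A one-shot trigger actor that rotates a referenced directional light to a desired rotation when BP_DustyCharacter enters its collision.
; On first valid overlap it captures the light's current rotation, resets its timer and enables Tick, which is otherwise disabled from BeginPlay.
; Tick lerps the light's rotation over a configurable duration, then turns itself off once complete.
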(event `self.ReceiveBeginPlay`
  (`self.SetActorTickEnabled` false))

(event `self.ReceiveTick`
  (params (DeltaSeconds :type "Float (single-precision)"))
  (bind _returnvalue (/ (`self.Alpha`) (`self.TimeForFullRot`)))
  (if (`self.Rotating`)
    (set `self.Alpha` (+ DeltaSeconds (`self.Alpha`)))
    (`self.K2_SetActorRotation` (`self.Directional Light`) (`KismetMathLibrary.RLerp` (`self.InitRotation`) (`self.Desired Rotation`) _returnvalue) false)
    (if (>= _returnvalue 1.0)
      (set `self.Rotating` false)
      (`self.SetActorTickEnabled` false))))

(event `self.CollisionComponent.OnComponentBeginOverlap`
  (params (OverlappedComponent :type "PrimitiveComponent Object Reference") (OtherActor :type "Actor Object Reference") (OtherComp :type "PrimitiveComponent Object Reference") (OtherBodyIndex :type Integer) (bFromSweep :type Boolean) (SweepResult :type "HitResult Structure (by ref)"))
  (bind (_returnvalue_location _returnvalue_rotation) (`KismetMathLibrary.BreakTransform` (`self.GetTransform` (`self.Directional Light`))))
  (if (`self.doOnce`)
    (`/Engine/EditorBlueprintResources/StandardMacros.IsValid` (`self.Directional Light`)
      (:`Is Valid`
        (if (`GameplayStatics.ObjectIsA` OtherActor "/Game/Blueprints/Characters/BP_DustyCharacter.BP_DustyCharacter_C")
          (set `self.doOnce` false)
          (set `self.Rotating` true)
          (set `self.Alpha` 0.0)
          (set `self.InitRotation` _returnvalue_rotation)
          (`self.SetActorTickEnabled` true))))))

(fn `UserConstructionScript`)